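; Single interactable door on a physics-simulated skeletal mesh, with a scripted, animated close.
; CloseDoor, unless already closing or closed, disables physics and captures the door bone's current pitch.
; A timeline drives ABP_Door's override pitch from that angle to just short of zero, then releases the override and restores physics.
; Tick optionally prints bone rotation for debugging; handle-alignment, bounds and blocker-disabling nodes are left unconnected.
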(event `self.ReceiveBeginPlay`
  (`parent.ReceiveBeginPlay`))

(event `self.ReceiveTick`
  (params (DeltaSeconds :type "Float (single-precision)"))
  (`parent.ReceiveTick` DeltaSeconds)
  (if (`self.DebugDoorBoneRot`)
    (`KismetSystemLibrary.PrintString` (`KismetStringLibrary.Conv_RotatorToString` (.rotation (`SkinnedMeshComponent.GetBoneTransform` (`self.DoorSkeletalMesh`) (`self.DoorBoneName`) "RTS_ParentBoneSpace"))))))

(event `CloseDoor`
  (bind _doorskeletalmesh (`self.DoorSkeletalMesh`))
  (if (not (or (`self.IsClosing`) (`self.IsClosed`)))
    (`KismetSystemLibrary.PrintString` "START COLSE TIMELINE")
    (bind _asabp_door (cast `/InteractiveDoorFramework/Core/Placeholders/Door/ABP_Door` (`SkeletalMeshComponent.GetAnimInstance` (`self.DoorSkeletalMesh`))))
    (`SkeletalMeshComponent.SetBodySimulatePhysics` _doorskeletalmesh (`self.DoorBoneName`) false)
    (`PrimitiveComponent.SetSimulatePhysics` _doorskeletalmesh false)
    (set `self.IsClosing` true)
    (`KismetSystemLibrary.Delay` 0.0)
    (set `self.InitialDoorPitch` (.pitch (.rotation (`SkinnedMeshComponent.GetBoneTransform` (`self.DoorSkeletalMesh`) (`self.DoorBoneName`) "RTS_ParentBoneSpace"))))
    (set `self.TotalAngleToAdd` (- (`self.InitialDoorPitch`) 0.0))
    (set `/InteractiveDoorFramework/Core/Placeholders/Door/ABP_Door.DoorOverrideAlpha` 1.0 _asabp_door)
    (bind (_direction _newtrack_0) (`Timeline|Timeline` :!via `PlayFromStart`)
      (:`Update`
        (set `/InteractiveDoorFramework/Core/Placeholders/Door/ABP_Door.DoorPitchToAdd` (`KismetMathLibrary.Lerp` (`self.TotalAngleToAdd`) 0.0 (* _newtrack_0 0.99)) _asabp_door))
      (:`Finished`
        (set `/InteractiveDoorFramework/Core/Placeholders/Door/ABP_Door.DoorOverrideAlpha` 0.0 _asabp_door)
        (`SkeletalMeshComponent.SetBodySimulatePhysics` (`self.DoorSkeletalMesh`) (`self.DoorBoneName`) true)
        (`PrimitiveComponent.SetSimulatePhysics` (`self.DoorSkeletalMesh`) true)
        (set `self.IsClosing` false)))))

(fn `UserConstructionScript`
  (`parent.UserConstructionScript`))