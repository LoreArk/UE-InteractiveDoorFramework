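; BP_DoubleDoor is an interactable door with two skeletal mesh leaves, each animated through an ABP_Door anim instance.
; On BeginPlay it runs the parent's logic, then passes each leaf's anim instance its own handle transform reference.
; It adds no other graph logic, so any interaction behavior comes from outside this Blueprint's graphs.
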(event `self.ReceiveBeginPlay`
  (`parent.ReceiveBeginPlay`)
  (`|ExecutionSequence`
    (:`then_0`
      (bind _asabp_door (cast `/InteractiveDoorFramework/Core/Placeholders/Door/ABP_Door` (`SkeletalMeshComponent.GetAnimInstance` (`self.DoorSkeletalMesh`))))
      (set `/InteractiveDoorFramework/Core/Placeholders/Door/ABP_Door.HandleTransform` (`self.HandleTransformRef`) _asabp_door))
    (:`then_1`
      (bind _asabp_door_2 (cast `/InteractiveDoorFramework/Core/Placeholders/Door/ABP_Door` (`SkeletalMeshComponent.GetAnimInstance` (`self.SecondDoorSkeletalMesh`))))
      (set `/InteractiveDoorFramework/Core/Placeholders/Door/ABP_Door.HandleTransform` (`self.HandleTransformRefB`) _asabp_door_2))))

(fn `UserConstructionScript`)